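; BP_Hero is the player character Blueprint for the Under The Well level, handling basic movement, camera look and jumping.
; Input Action events drive forward and right movement along vectors derived from control rotation, with pitch zeroed to keep movement independent of look pitch.
; Turn and look-up actions feed controller yaw and pitch, while the jump action calls Jump.
; The construction script is empty.
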(event `EnhancedInput|/Game/BluePrints/LevelUnderTheWell/Player/Input/IA_MoveForward`
  (params (ActionValue :type "Float (double-precision)") (ElapsedSeconds :type "Float (double-precision)") (TriggeredSeconds :type "Float (double-precision)") (InputAction :type "InputAction Object Reference" :default "/Game/BluePrints/LevelUnderTheWell/Player/Input/IA_MoveForward.IA_MoveForward"))
  (bind (_returnvalue_roll _returnvalue_pitch _returnvalue_yaw) (`KismetMathLibrary.BreakRotator` (`self.GetControlRotation`)))
  ;[1 1 1] Movement
  (:`Triggered`
    (`self.AddMovementInput` (`KismetMathLibrary.GetForwardVector` (`KismetMathLibrary.MakeRotator` 0.0 0.0 _returnvalue_yaw)) ActionValue)))

(event `EnhancedInput|/Game/BluePrints/LevelUnderTheWell/Player/Input/IA_Turn`
  (params (ActionValue :type "Float (double-precision)") (ElapsedSeconds :type "Float (double-precision)") (TriggeredSeconds :type "Float (double-precision)") (InputAction :type "InputAction Object Reference" :default "/Game/BluePrints/LevelUnderTheWell/Player/Input/IA_Turn.IA_Turn"))
  ;[1 1 1] Camera Movement
  (:`Triggered`
    (`self.AddControllerYawInput` ActionValue)))

(event `EnhancedInput|/Game/BluePrints/LevelUnderTheWell/Player/Input/IA_LookUp`
  (params (ActionValue :type "Float (double-precision)") (ElapsedSeconds :type "Float (double-precision)") (TriggeredSeconds :type "Float (double-precision)") (InputAction :type "InputAction Object Reference" :default "/Game/BluePrints/LevelUnderTheWell/Player/Input/IA_LookUp.IA_LookUp"))
  ;[1 1 1] Camera Movement
  (:`Triggered`
    (`self.AddControllerPitchInput` ActionValue)))

(event `EnhancedInput|/Game/BluePrints/LevelUnderTheWell/Player/Input/IA_MoveRight`
  (params (ActionValue :type "Float (double-precision)") (ElapsedSeconds :type "Float (double-precision)") (TriggeredSeconds :type "Float (double-precision)") (InputAction :type "InputAction Object Reference" :default "/Game/BluePrints/LevelUnderTheWell/Player/Input/IA_MoveRight.IA_MoveRight"))
  (bind (_returnvalue_roll _returnvalue_pitch _returnvalue_yaw) (`KismetMathLibrary.BreakRotator` (`self.GetControlRotation`)))
  ;[1 1 1] Movement
  (:`Triggered`
    (`self.AddMovementInput` (`KismetMathLibrary.GetRightVector` (`KismetMathLibrary.MakeRotator` _returnvalue_roll 0.0 _returnvalue_yaw)) ActionValue)))

(event `EnhancedInput|/Game/BluePrints/LevelUnderTheWell/Player/Input/IA_Jump`
  (params (ActionValue :type Boolean) (ElapsedSeconds :type "Float (double-precision)") (TriggeredSeconds :type "Float (double-precision)") (InputAction :type "InputAction Object Reference" :default "/Game/BluePrints/LevelUnderTheWell/Player/Input/IA_Jump.IA_Jump"))
  (:`Triggered`
    (`self.Jump`)))

(fn `UserConstructionScript`)